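; Wardrobe actor that the player can enter and leave with E, moving the pawn inside and switching the view to the armoire.
; Box overlap shows a prompt widget, saves the pawn's location and starts two looping timers that poll the character's E-press flag.
; Entering sets IsIn after a short delay; exiting restores the saved location and character view.
; Each timer clears when its action fires; end overlap only removes the widget.
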(event OnComponentBeginOverlap(Box)
  (params (OverlappedComponent :type Primitive%20Component%20Object%20Reference) (OtherActor :type Actor%20Object%20Reference) (OtherComp :type Primitive%20Component%20Object%20Reference) (OtherBodyIndex :type Integer) (bFromSweep :type Boolean) (SweepResult :type Hit%20Result%20Structure%20%28by%20ref%29))
  (bind _asthird_person_character_clem (Utilities|Casting|CastToThirdPersonCharacterClem OtherActor))
  (Variables|Default|SetThird_Person_Ref _asthird_person_character_clem)
  (bind _returnvalue (UserInterface|CreateWidget "/Game/DEV/Widgets/Player_UI/Armoire_UI.Armoire_UI_C"))
  (bind _output_get (Variables|Default|SetArmoire_UI _returnvalue))
  (UserInterface|Viewport|AddtoViewport _output_get 0)
  (Variables|Default|SetActor_Location_Save (Transformation|GetActorLocation (Game|Player|GetPlayerPawn 0)))
  (Utilities|FlowControl|Sequence
    (:then_0
      (bind _returnvalue_2 (Utilities|Time|SetTimerbyEvent (delegate Custom|Armoire_IN/OUT) 0.01 true)))
    (:then_1
      (bind _returnvalue_3 (Utilities|Time|SetTimerbyEvent (delegate Custom|Armoire_out) 0.01 true)))))

(event OnComponentEndOverlap(Box)
  (params (OverlappedComponent :type Primitive%20Component%20Object%20Reference) (OtherActor :type Actor%20Object%20Reference) (OtherComp :type Primitive%20Component%20Object%20Reference) (OtherBodyIndex :type Integer))
  (Widget|RemovefromParent (Variables|Default|GetArmoire_UI)))

(event Custom|Armoire_IN/OUT
  (if (Variables|/Game/DEV/ThirdPersonBP/Blueprints/ThirdPersonCharacterClem.ThirdPersonCharacterClem_C|GetIsEPressed? (Variables|Default|GetThird_Person_Ref))
    (Transformation|SetActorLocation (Game|Player|GetPlayerPawn 0) (Transformation|GetActorLocation) false false)
    (Game|Player|SetViewTargetwithBlend (Game|GetPlayerController 0) self 0.0 "VTBlend_Linear" 0.0 false)
    (Widget|RemovefromParent (Variables|Default|GetArmoire_UI))
    (Utilities|FlowControl|Delay 0.5)
    (Variables|Default|SetIsIn? true)
    (Utilities|Time|ClearandInvalidateTimerbyHandle (stale OnComponentBeginOverlap(Box) _returnvalue_2))))

(event Custom|Armoire_out
  (if (and (Variables|/Game/DEV/ThirdPersonBP/Blueprints/ThirdPersonCharacterClem.ThirdPersonCharacterClem_C|GetIsEPressed? (Variables|Default|GetThird_Person_Ref)) (Variables|Default|GetIsIn?))
    (Transformation|SetActorLocation (Game|Player|GetPlayerPawn 0) (Variables|Default|GetActor_Location_Save) false false)
    (Game|Player|SetViewTargetwithBlend (Game|GetPlayerController 0) (Variables|Default|GetThird_Person_Ref) 0.0 "VTBlend_Linear" 0.0 false)
    (Variables|Default|SetIsIn? false)
    (Utilities|Time|ClearandInvalidateTimerbyHandle (stale OnComponentBeginOverlap(Box) _returnvalue_3))))

(fn ConstructionScript)